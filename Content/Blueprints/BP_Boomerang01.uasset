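; BP_Boomerang01 is a thrown boomerang projectile that damages enemies and returns to the player's hand.
; It turns back two seconds after spawning or when its box overlaps another actor, which also spawns a Niagara effect and damages BP_EnemyAI.
; The return zeroes gravity, then a timeline lerps it to the character's Boomerang component.
; On arrival it plays a catch sound, destroys itself and calls ResetBoom on the character.
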(event `self.ReceiveBeginPlay`
  ;[0.15 0.147 0.01229 0.502] Boomerang returning to the player (I think...) (Maybe someone can fill this comment out if they have more info?)
  (set `self.PlayerCharacter` (`GameplayStatics.GetPlayerPawn` (`self.Player Index`)))
  (`KismetSystemLibrary.Delay` 2.0)
  (if (not (`self.IsReturning`))
    (`self.BoomReturn`)))

(event `BoomReturn`
  (bind _asbp_third_person_character (cast `/Game/Blueprints/BP_ThirdPersonCharacter` (`GameplayStatics.GetPlayerCharacter` 0) :!pure true))
  ;[0.15 0.147 0.01229 0.502] Boomerang Returning to Player
  (set `self.IsReturning` true)
  (set `ProjectileMovementComponent.ProjectileGravityScale` 0.0 (`self.ProjectileMovement`))
  (`KismetSystemLibrary.Delay` 0.1)
  (set `self.BoomLocBegin` (`self.K2_GetActorLocation` self))
  (bind (_direction _boomreturn) (`Timeline|BoomerangReturn`)
    (:`Update`
      (`self.K2_SetActorLocation` (`KismetMathLibrary.VLerp` (`self.BoomLocBegin`) (`SceneComponent.K2_GetComponentLocation` (`/Game/Blueprints/BP_ThirdPersonCharacter.Boomerang` _asbp_third_person_character)) _boomreturn)))
    (:`Finished`
      ;;[0 0.0319 0.15 0.502] Playing Returning Boomerang SFX
      (bind _returnvalue (`GameplayStatics.SpawnSound2D` "/Game/Sounds/SFX/Boomerang_SFX/Catch_Cardboard_Box_1_SFX.Catch_Cardboard_Box_1_SFX" 0.5 0.75 0.0 null))
      (`KismetSystemLibrary.PrintString` (`KismetSystemLibrary.GetDisplayName` _returnvalue))
      (`self.K2_DestroyActor`)
      (`/Game/Blueprints/BP_ThirdPersonCharacter.ResetBoom` _asbp_third_person_character))))

(event `self.Box.OnComponentBeginOverlap`
  (params (OverlappedComponent :type "PrimitiveComponent Object Reference") (OtherActor :type "Actor Object Reference") (OtherComp :type "PrimitiveComponent Object Reference") (OtherBodyIndex :type Integer) (bFromSweep :type Boolean) (SweepResult :type "HitResult Structure (by ref)"))
  (bind (_asbp_enemy_ai _bsuccess) (cast `/Game/Blueprints/BP_EnemyAI` OtherActor :!pure true))
  ;[0.1458 0.00185 0 0.5] When the Boomerang overlaps with the Enemy
  (if (== OtherActor self)
    _
    (elif (not (== OtherActor (`GameplayStatics.GetPlayerCharacter` 0)))
      (`KismetSystemLibrary.PrintString` (`KismetSystemLibrary.GetDisplayName` OtherActor))
      (`|ExecutionSequence`
        (:`then_0`
          (`self.BoomReturn`))
        (:`then_1`
          (`NiagaraFunctionLibrary.SpawnSystemAtLocation` "/Game/Effects/NS_BoomSystem.NS_BoomSystem" (`self.K2_GetActorLocation`)))
        (:`then_2`
          (if _bsuccess
            (`KismetSystemLibrary.PrintString` "True")
            (`/Engine/EditorBlueprintResources/StandardMacros.IsValid` _asbp_enemy_ai
              (:`Is Valid`
                (`/Game/Blueprints/BP_EnemyAI.DecreaseHealth` _asbp_enemy_ai (`self.Boomerang DMG`)) ; Boomerang decresasing the Enemy's Health
              ))
            (else
              (`KismetSystemLibrary.PrintString` "False"))))))))

(fn `ReturnToPlayer`)

(fn `UserConstructionScript`)