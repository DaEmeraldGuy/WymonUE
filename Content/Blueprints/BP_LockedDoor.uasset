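; BP_LockedDoor is a locked door actor that removes itself when a player character holding a key reaches it.
; A TriggerBox overlap casts to BP_ThirdPersonCharacter, then checks the "player" tag and the HasKey flag.
; A timeline then drives the scale of the Lock, Cone and Sphere components.
; Its update also starts a short delay, after which the whole actor is destroyed.
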(event `self.Trigger Box.OnComponentBeginOverlap`
  (params (OverlappedComponent :type "PrimitiveComponent Object Reference") (OtherActor :type "Actor Object Reference") (OtherComp :type "PrimitiveComponent Object Reference") (OtherBodyIndex :type Integer) (bFromSweep :type Boolean) (SweepResult :type "HitResult Structure (by ref)"))
  ;[0.28 1 0.2967] Condition (has key)
  (bind _asbp_third_person_character (cast `/Game/Blueprints/BP_ThirdPersonCharacter` OtherActor))
  (if (`self.ActorHasTag` OtherActor "player")
    (if (`/Game/Blueprints/BP_ThirdPersonCharacter.Has Key?` _asbp_third_person_character)
      ;[1 0.8408 0.1661] Animation
      (bind (_direction _newtrack_0) (`Timeline|Timeline`)
        (:`Update`
          (`SceneComponent.SetRelativeScale3D` (`self.Lock`) _newtrack_0)
          (`SceneComponent.SetRelativeScale3D` (`self.Cone`) _newtrack_0)
          (`SceneComponent.SetRelativeScale3D` (`self.Sphere`) _newtrack_0)
          (`KismetSystemLibrary.Delay` 1.2)
          (`self.K2_DestroyActor`))))))

(fn `UserConstructionScript`)