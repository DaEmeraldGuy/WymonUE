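; BP_Campfire is a checkpoint actor that lights up when the player character reaches it.
; A box overlap clears IsLastCampfire on every campfire, then, for BP_ThirdPersonCharacter, marks itself as last, stores itself in the game mode's LastCampfire and turns on its Niagara effect and light.
; Tick keeps any campfire that is not the last one dark by hiding the effect and zeroing the light.
; The flag reset runs before the character cast, so any overlapping actor clears it.
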(event `self.Box.OnComponentBeginOverlap`
  (params (OverlappedComponent :type "PrimitiveComponent Object Reference") (OtherActor :type "Actor Object Reference") (OtherComp :type "PrimitiveComponent Object Reference") (OtherBodyIndex :type Integer) (bFromSweep :type Boolean) (SweepResult :type "HitResult Structure (by ref)"))
  (bind _outactors (`GameplayStatics.GetAllActorsOfClass` "BP_Campfire_C"))
  (for _array_element _outactors
    (set `/Game/Blueprints/BP_Campfire.IsLastCampfire?` false _array_element))
  (cast `/Game/Blueprints/BP_ThirdPersonCharacter` OtherActor)
  (bind _asbp_third_person_game_mode (cast `/Game/ThirdPerson/Blueprints/BP_ThirdPersonGameMode` (`GameplayStatics.GetGameMode`)))
  (set `/Game/ThirdPerson/Blueprints/BP_ThirdPersonGameMode.Last Campfire` self _asbp_third_person_game_mode)
  (set `self.IsLastCampfire?` true)
  (`SceneComponent.SetVisibility` (`self.Niagara`) true false)
  (`LightComponent.SetIntensity` (`self.camp light`) 200000.0))

(event `self.ReceiveTick`
  (params (DeltaSeconds :type "Float (single-precision)"))
  (if (not (`self.IsLastCampfire?`))
    (`SceneComponent.SetVisibility` (`self.Niagara`) false false)
    (`LightComponent.SetIntensity` (`self.camp light`) 0.0)))

(fn `UserConstructionScript`)