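; BP_FireTornado is a short-lived projectile hazard that damages birds inside its box and destroys itself a few seconds after spawning.
; Each Tick it polls the box for overlapping BP_Bird actors and calls DecreaseHealth on one.
; A single ImmuneFrames flag, cleared after a Delay, throttles damage across all overlapping birds rather than per bird.
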(event `self.ReceiveBeginPlay`
  (`KismetSystemLibrary.Delay` 3.0)
  (`self.K2_DestroyActor`))

(event `self.ReceiveTick`
  (params (DeltaSeconds :type "Float (single-precision)"))
  (for _array_element (`PrimitiveComponent.GetOverlappingActors` (`self.Box`) "/Game/Blueprints/Enemies/BP_Bird.BP_Bird_C")
    (if (not (`self.ImmuneFrames`))
      (bind _asbp_bird (cast `/Game/Blueprints/Enemies/BP_Bird` _array_element))
      (`/Game/Blueprints/Enemies/BP_Bird.DecreaseHealth` _asbp_bird 2) ; Boomerang decresasing the Enemy's Health
      (set `self.ImmuneFrames` true)
      (`KismetSystemLibrary.Delay` 0.4)
      (set `self.ImmuneFrames` false))))

(fn `UserConstructionScript`)