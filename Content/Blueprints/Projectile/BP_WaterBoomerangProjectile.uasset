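; Water boomerang projectile that flies out, then returns to the player after a short timeout or on hitting something other than the player.
; After a brief overlap delay, the first Enemy-tagged hit spawns a BP_FireTornado at that actor and triggers the return.
; The return uses a Timeline to lerp toward the character's current location without sweep, then plays a catch sound, destroys the projectile and calls ResetBoom on the character.
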(event `self.ReceiveBeginPlay`
  ;[0.15 0.03203 0.03203 0.5] Check if returning
  (set `self.Player Character` (`GameplayStatics.GetPlayerPawn` 0))
  (`KismetSystemLibrary.Delay` 0.75)
  (if (not (`self.BoomerangReturning`))
    (`self.Boomerang Returning`)))

(event `Boomerang Returning`
  ;[0.04647 0.15 0.06769 0.5] Return to Player
  (set `self.BoomerangReturning` true)
  (bind _asbp_third_person_character (cast `/Game/Blueprints/BP_ThirdPersonCharacter` (`GameplayStatics.GetPlayerCharacter` 0)))
  (bind (_direction _return) (`Timeline|Timeline`)
    (:`Update`
      (`self.K2_SetActorLocation` (`KismetMathLibrary.VLerp` (`self.K2_GetActorLocation`) (`SceneComponent.K2_GetComponentLocation` (`Actor.RootComponent` _asbp_third_person_character)) _return)))
    (:`Finished`
      (`GameplayStatics.SpawnSound2D` "/Game/Sounds/SFX/Boomerang_SFX/Catch_Cardboard_Box_1_SFX.Catch_Cardboard_Box_1_SFX" 0.5 0.75 0.0 null)
      (`self.K2_DestroyActor`)
      (`/Game/Blueprints/BP_ThirdPersonCharacter.ResetBoom` _asbp_third_person_character))))

(event `self.Hitbox.OnComponentBeginOverlap`
  (params (OverlappedComponent :type "PrimitiveComponent Object Reference") (OtherActor :type "Actor Object Reference") (OtherComp :type "PrimitiveComponent Object Reference") (OtherBodyIndex :type Integer) (bFromSweep :type Boolean) (SweepResult :type "HitResult Structure (by ref)"))
  ;[0.15 0.1313 0.04447 0.5] Collision
  (`KismetSystemLibrary.Delay` 0.2)
  (if (`self.ActorHasTag` OtherActor "Enemy")
    (`/Engine/EditorBlueprintResources/StandardMacros.DoOnce` false
      (:`Completed`
        (`|SpawnActorFromClass` "/Game/Blueprints/Projectile/BP_FireTornado.BP_FireTornado_C" (`KismetMathLibrary.MakeTransform` (`self.K2_GetActorLocation` OtherActor)) "Undefined" "MultiplyWithRoot" null null)
        (`self.Boomerang Returning`)))
    (elif (not (`self.ActorHasTag` OtherActor "Player"))
      (`self.Boomerang Returning`))))

(fn `UserConstructionScript`)