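; BP_NPC is an NPC that shows named dialogue lines in a W_Dialogue widget.
; Each Talk call steps through the Dialogue and Name arrays, plays a pop sound, and removes the widget when either runs out.
; A one-time trigger overlap starts Talk unless the GameMode's SeenDoorTalk flag is set, briefly toggling input.
; Player contact with CollisionBox sets the NPC's ground friction very high.
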(event `/Game/Blueprints/BPI_Dialogue.Talk`
  (`/Engine/EditorBlueprintResources/StandardMacros.IncrementInt` (`self.TalkIndex`)
    (:`  `
      (if (< (`self.TalkIndex`) (`KismetArrayLibrary.Array_Length` (`self.Dialogue`)))
        (`/Engine/EditorBlueprintResources/StandardMacros.IncrementInt` (`self.NameIndex`)
          (:`  `
            (if (< (`self.NameIndex`) (`KismetArrayLibrary.Array_Length` (`self.Name`)))
              (`self.W_Dialogue`
                (:`then`
                  _)
                (:`else`
                  (bind _returnvalue (`|CreateWidget` "/Game/Sequences/Writing_NarrativeUI/W_Dialogue.W_Dialogue_C" (`GameplayStatics.GetPlayerController` 0)))
                  (bind _output_get (set `self.W_Dialogue` _returnvalue))
                  (`UserWidget.AddToViewport` _output_get 0)))
              (`TextBlock.SetText` (`/Game/Sequences/Writing_NarrativeUI/W_Dialogue.TalkText` (`self.W_Dialogue`)) (`KismetTextLibrary.Conv_StringToText` (`|GetArrayItem` (`self.Dialogue`) (`self.TalkIndex`))))
              (`TextBlock.SetText` (`/Game/Sequences/Writing_NarrativeUI/W_Dialogue.NameText` (`self.W_Dialogue`)) (`KismetTextLibrary.Conv_StringToText` (`|GetArrayItem` (`self.Name`) (`self.NameIndex`))))
              (`GameplayStatics.PlaySound2D` "/Game/Sounds/SFX/Pop_SFX/Pop_1.Pop_1" 1.0 1.0 0.0 null null) ; Plays "Pop_1" SFX when new text appear
              (else
                (`Widget.RemoveFromParent` (`self.W_Dialogue`))))))
        (else
          (`Widget.RemoveFromParent` (`self.W_Dialogue`)))))))

(event `self.DialogueTrigger.OnComponentBeginOverlap`
  (params (OverlappedComponent :type "PrimitiveComponent Object Reference") (OtherActor :type "Actor Object Reference") (OtherComp :type "PrimitiveComponent Object Reference") (OtherBodyIndex :type Integer) (bFromSweep :type Boolean) (SweepResult :type "HitResult Structure (by ref)"))
  (bind _returnvalue (`GameplayStatics.GetPlayerController` OtherBodyIndex))
  (`/Engine/EditorBlueprintResources/StandardMacros.DoOnce` false
    (:`Completed`
      (bind _asbp_third_person_game_mode (cast `/Game/ThirdPerson/Blueprints/BP_ThirdPersonGameMode` (`GameplayStatics.GetGameMode`)))
      (if (not (`/Game/ThirdPerson/Blueprints/BP_ThirdPersonGameMode.Seen Door Talk?` _asbp_third_person_game_mode))
        (`self.DisableInput` OtherActor _returnvalue)
        (`self.Talk`)
        (bind _asbp_third_person_game_mode_2 (cast `/Game/ThirdPerson/Blueprints/BP_ThirdPersonGameMode` (`GameplayStatics.GetGameMode`)))
        (set `/Game/ThirdPerson/Blueprints/BP_ThirdPersonGameMode.Seen Door Talk?` true _asbp_third_person_game_mode_2)
        (`self.EnableInput` OtherActor _returnvalue)))))

(event `self.CollisionBox.OnComponentBeginOverlap`
  (params (OverlappedComponent :type "PrimitiveComponent Object Reference") (OtherActor :type "Actor Object Reference") (OtherComp :type "PrimitiveComponent Object Reference") (OtherBodyIndex :type Integer) (bFromSweep :type Boolean) (SweepResult :type "HitResult Structure (by ref)"))
  (cast `/Game/Blueprints/BP_ThirdPersonCharacter` OtherActor)
  (set `CharacterMovementComponent.GroundFriction` 100.0 (`self.CharacterMovement`)))

(fn `UserConstructionScript`)