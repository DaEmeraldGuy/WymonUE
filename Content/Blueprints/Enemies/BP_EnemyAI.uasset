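; Enemy character that chases the player, takes damage and displays a health bar above it.
; PawnSensing sight triggers an AIMoveTo toward the player, with no logic here to clear the seen flag.
; DecreaseHealth applies clamped damage with brief immunity frames, broadcasts the change, then at zero notifies ArenaDoors and destroys the enemy.
; Tick updates the widget's bar, re-initialises and rebroadcasts health, and turns it toward the camera.
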(event `self.ReceiveBeginPlay`
  ; Testing
)

(event `self.ReceiveTick`
  (params (DeltaSeconds :type "Float (single-precision)"))
  (bind _enemy_health_bar_widget (`self.Enemy Health Bar Widget`))
  ;[0.2122 0.0137 0.0137 0.502] Updating Enemy Health Bar
  (bind _aswbp_enemy_health_bar (cast `/Game/UI_Design/WBP_Enemy_HealthBar` (`WidgetComponent.GetWidget` (`self.Enemy Health Bar Widget`))))
  (`ProgressBar.SetPercent` (`/Game/UI_Design/WBP_Enemy_HealthBar.EnemyHealthBar` _aswbp_enemy_health_bar) (/ (`KismetMathLibrary.Conv_IntToDouble` (`self.Current Health`)) (`KismetMathLibrary.Conv_IntToDouble` (`self.Max Health`))))
  (`|ExecutionSequence`
    (:`then_0`
      ;;[0.6667 0.5549 0.2377 0.5] Health Bar Following the Camera
      (`SceneComponent.K2_SetWorldRotation` _enemy_health_bar_widget (`KismetMathLibrary.FindLookAtRotation` (`SceneComponent.K2_GetComponentLocation` _enemy_health_bar_widget) (`SceneComponent.K2_GetComponentLocation` (`PlayerCameraManager.TransformComponent` (`GameplayStatics.GetPlayerCameraManager` 0)))) false false))
    (:`then_1`
      ;;[0.6654 0.2789 0.2789 0.502] Updating the Enemy's HP Text Number
      (`/Game/UI_Design/WBP_Enemy_HealthBar.Initialise Enemy Health` _aswbp_enemy_health_bar self)
      (`self.Enemy_HealthUpdated` (`self.Current Health`) (`self.Max Health`)))))

(event `DecreaseHealth`
  (params (Damage :type Integer))
  ;[0.2122 0.0137 0.0137 0.502] Enemy Damage System
  (if (not (`self.ImmunityFrames`))
    (set `self.ImmunityFrames` true)
    (bind _output_get (set `self.Current Health` (`KismetMathLibrary.FTrunc` (`KismetMathLibrary.FClamp` (`KismetMathLibrary.Conv_IntToDouble` (- (`self.Current Health`) Damage)) 0.0 100.0))))
    (`self.Enemy_HealthUpdated` _output_get (`self.Max Health`))
    (`KismetSystemLibrary.Delay` 0.25)
    (set `self.ImmunityFrames` false)
    (if (<= _output_get 0)
      (message `/Game/Blueprints/EnemyDies.EnemyDies` (`self.ArenaDoors`))
      (`self.K2_DestroyActor`))))

(event `self.PawnSensing.OnSeePawn`
  (params (Pawn :type "Pawn Object Reference"))
  ;[0.15 0.1217 0.000781 0.5] Enemy Following the Player (AI)
  (set `self.isSeeingPlayer` true)
  (`self.FollowPlayer`))

(event `FollowPlayer`
  ;[0.15 0.1217 0.000781 0.5] Enemy Following the Player (AI)
  (`KismetSystemLibrary.PrintString` "Enemy: Player in sight!" true true (struct :`R` 1.0 :`G` 0.056447 :`B` 0.065997 :`A` 1.0))
  (if (`self.isSeeingPlayer`)
    (`|AIMoveTo` self (0.0 0.0 0.0) (`GameplayStatics.GetPlayerCharacter` 0))))

(fn `UserConstructionScript`)