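; Bird enemy that chases the player on sight, deals contact damage, and notifies ArenaDoors before destroying itself at zero health.
; PawnSensing triggers AIMoveTo toward the player; while patrolling without sight, Tick rotates it 180 degrees after a delay, and roaming logic is disconnected.
; Tick also updates its health bar widget and turns it toward the camera.
; One ImmunityFrames flag, cleared by delays, throttles both damage taken and dealt.
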(event `self.ReceiveTick`
  (params (DeltaSeconds :type "Float (single-precision)"))
  (bind _enemy_health_bar_widget (`self.Enemy Health Bar Widget`))
  ;[0.2122 0.0137 0.0137 0.502] Updating Enemy Health Bar
  (`|ExecutionSequence`
    (:`then_0`
      (bind _aswbp_enemy_health_bar (cast `/Game/UI_Design/WBP_Enemy_HealthBar` (`WidgetComponent.GetWidget` (`self.Enemy Health Bar Widget`))))
      (`ProgressBar.SetPercent` (`/Game/UI_Design/WBP_Enemy_HealthBar.EnemyHealthBar` _aswbp_enemy_health_bar) (/ (`KismetMathLibrary.Conv_IntToDouble` (`self.Current Health`)) (`KismetMathLibrary.Conv_IntToDouble` (`self.Max Health`))))
      (`|ExecutionSequence`
        (:`then_0`
          ;;[0.6667 0.5549 0.2377 0.5] Health Bar Following the Camera
          (`SceneComponent.K2_SetWorldRotation` _enemy_health_bar_widget (`KismetMathLibrary.FindLookAtRotation` (`SceneComponent.K2_GetComponentLocation` _enemy_health_bar_widget) (`SceneComponent.K2_GetComponentLocation` (`PlayerCameraManager.TransformComponent` (`GameplayStatics.GetPlayerCameraManager` 0)))) false false))
        (:`then_1`
          ;;[0.6654 0.2789 0.2789 0.502] Updating the Enemy's HP Text Number
          (`/Game/UI_Design/WBP_Enemy_HealthBar.Initialise Enemy Health` _aswbp_enemy_health_bar self)
          (`self.Enemy_HealthUpdated` (`self.Current Health`) (`self.Max Health`)))))
    (:`then_1`
      ;[0.15 0.1217 0.000781 0.5] Enemy Following the Player (AI)
      (if (`self.isPatroling`)
        (if (not (`self.isSeeingPlayer`))
          (`KismetSystemLibrary.Delay` 1.5)
          (if (`self.isPatroling`)
            (`self.K2_AddActorLocalRotation` self (struct :`Yaw` 180.0) false false)))))))

(event `DecreaseHealth`
  (params (Damage :type Integer))
  ;[0.2122 0.0137 0.0137 0.502] Enemy Damage System
  (if (not (`self.ImmunityFrames`))
    (set `self.ImmunityFrames` true)
    (bind _output_get (set `self.Current Health` (`KismetMathLibrary.FTrunc` (`KismetMathLibrary.FClamp` (`KismetMathLibrary.Conv_IntToDouble` (- (`self.Current Health`) Damage)) 0.0 100.0))))
    (`self.Enemy_HealthUpdated` _output_get (`self.Max Health`))
    (`KismetSystemLibrary.Delay` 0.25)
    (set `self.ImmunityFrames` false)
    (if (<= _output_get 0)
      (message `/Game/Blueprints/EnemyDies.EnemyDies` (`self.ArenaDoors`))
      (`self.K2_DestroyActor`))))

(event `self.PawnSensing.OnSeePawn`
  (params (Pawn :type "Pawn Object Reference"))
  ;[0.15 0.1217 0.000781 0.5] Enemy Following the Player (AI)
  (set `self.isSeeingPlayer` true)
  (`self.FollowPlayer`))

(event `FollowPlayer`
  ;[0.15 0.1217 0.000781 0.5] Enemy Following the Player (AI)
  (if (`self.isSeeingPlayer`)
    (`|AIMoveTo` self (0.0 0.0 0.0) (`GameplayStatics.GetPlayerCharacter` 0)
      (:`OnSuccess`
        (set `self.isSeeingPlayer` true)
        (set `self.isPatroling` false))
      (:`OnFail`
        (set `self.isSeeingPlayer` false)
        (if (not (`self.isPatroling`))
          (set `self.isPatroling` true))))))

(event `self.CapsuleComponent.OnComponentHit`
  (params (HitComponent :type "PrimitiveComponent Object Reference") (OtherActor :type "Actor Object Reference") (OtherComp :type "PrimitiveComponent Object Reference") (NormalImpulse :type "Vector Structure") (Hit :type "HitResult Structure (by ref)"))
  ;[0.03028 0.15 0.05393 0.5] Damager
  (if (not (`self.ImmunityFrames`))
    (`GameplayStatics.ApplyDamage` OtherActor 2.0)
    (set `self.ImmunityFrames` true)
    (`KismetSystemLibrary.Delay` 2.0)
    (set `self.ImmunityFrames` false)))

(event `Roam`
  ; Roaming AI
)

(event `self.ReceiveBeginPlay`
  ; Roaming AI
)

(fn `UserConstructionScript`)