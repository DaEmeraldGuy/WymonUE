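; BP_CombatArena is a combat arena that shuts its front gate on the player and reopens it once all enemies are defeated.
; When the player character overlaps the trigger, a timeline lerps the gate down from its starting position, unless the arena is active or completed.
; EnemyDies counts kills until they match EnemyCount, then a second timeline raises the gate and marks completion.
; ArenaActive is never set here, and ActivateArena is empty.
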(event `self.ReceiveBeginPlay`
  ; Set Gate Beginning and End Location
  (bind _output_get (set `self.DoorBeginLoc` (`SceneComponent.RelativeLocation` (`self.Gate_Front`))))
  (set `self.DoorEndLoc` (`KismetMathLibrary.MakeVector` (.x _output_get) (.y _output_get) (+ (.z _output_get) -300.0))))

(event `self.TriggerVolume.OnComponentBeginOverlap`
  (params (OverlappedComponent :type "PrimitiveComponent Object Reference") (OtherActor :type "Actor Object Reference") (OtherComp :type "PrimitiveComponent Object Reference") (OtherBodyIndex :type Integer) (bFromSweep :type Boolean) (SweepResult :type "HitResult Structure (by ref)"))
  ; Front Gate Triggers when Player Character walks through triggger
  (cast `/Game/Blueprints/BP_ThirdPersonCharacter` OtherActor)
  (if (and (not (`self.bArenaCompleted`)) (not (`self.bArenaActive`)))
    (bind (_direction _doorclose) (`Timeline|ActivateGate`)
      (:`Update`
        (`SceneComponent.K2_SetRelativeLocation` (`self.Gate_Front`) (`KismetMathLibrary.VLerp` (`self.DoorBeginLoc`) (`self.DoorEndLoc`) _doorclose) false false)))))

(event `/Game/Blueprints/EnemyDies.EnemyDies`
  ; Counting Enemies in Battle Arena
  (`KismetSystemLibrary.PrintString` "Dead!!!")
  (set `self.EnemiesDefeated` (+ (`self.EnemiesDefeated`) 1))
  (if (== (`self.EnemiesDefeated`) (`self.EnemyCount`))
    (bind (_direction _doorclose) (`Timeline|Timeline`)
      (:`Update`
        (`SceneComponent.K2_SetRelativeLocation` (`self.Gate_Front`) (`KismetMathLibrary.VLerp` (`self.DoorEndLoc`) (`self.DoorBeginLoc`) _doorclose) false false)
        (set `self.bArenaCompleted` true)))))

(fn `ActivateArena`)

(fn `UserConstructionScript`)