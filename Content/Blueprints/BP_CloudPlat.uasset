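; BP_CloudPlat is a cloud platform that moves from StartPos to EndPos when an actor overlaps its trigger, then returns.
; A timeline lerps the platform's relative location while the third-person character's input is disabled.
; At arrival, input returns, and after a delay a second timeline plays in reverse.
; CanOverlap blocks retriggers until the return finishes, but is cleared before the character cast, so other actors lock it.
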(event `self.Trigger.OnComponentBeginOverlap`
  (params (OverlappedComponent :type "PrimitiveComponent Object Reference") (OtherActor :type "Actor Object Reference") (OtherComp :type "PrimitiveComponent Object Reference") (OtherBodyIndex :type Integer) (bFromSweep :type Boolean) (SweepResult :type "HitResult Structure (by ref)"))
  (bind _returnvalue (`GameplayStatics.GetPlayerController` 0))
  (if (`self.Can Overlap`)
    (set `self.Can Overlap` false)
    (bind _asbp_third_person_character (cast `/Game/Blueprints/BP_ThirdPersonCharacter` OtherActor))
    (`self.DisableInput` _asbp_third_person_character _returnvalue)
    (bind (_direction _newtrack_0) (`Timeline|Timeline` :!via `PlayFromStart`)
      (:`Update`
        (`SceneComponent.K2_SetRelativeLocation` (`self.Platform`) (`KismetMathLibrary.VLerp` (`self.Start Pos`) (`self.End Pos`) _newtrack_0) false false))
      (:`Finished`
        (`self.EnableInput` _asbp_third_person_character _returnvalue)
        (`KismetSystemLibrary.Delay` 3.0)
        (bind (_direction_2 _newtrack_0_2) (`Timeline|Timeline_0` :!via `ReverseFromEnd`)
          (:`Update`
            (`SceneComponent.K2_SetRelativeLocation` (`self.Platform`) (`KismetMathLibrary.VLerp` (`self.Start Pos`) (`self.End Pos`) _newtrack_0_2) false false))
          (:`Finished`
            (set `self.Can Overlap` true)))))))

(fn `UserConstructionScript`)