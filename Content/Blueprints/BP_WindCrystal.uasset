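; BP_WindCrystal is the Air Crystal pickup, collected when the third-person character overlaps its box.
; The overlap plays a one-shot 2D sound before the character cast, so the first overlapping actor of any kind triggers it.
; It then disables player input, calls WindCrystalGet on the character, waits briefly, sends BreakCloudMessage to two referenced clouds and destroys itself.
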(event `self.Box.OnComponentBeginOverlap`
  (params (OverlappedComponent :type "PrimitiveComponent Object Reference") (OtherActor :type "Actor Object Reference") (OtherComp :type "PrimitiveComponent Object Reference") (OtherBodyIndex :type Integer) (bFromSweep :type Boolean) (SweepResult :type "HitResult Structure (by ref)"))
  ;[0.04521 0.1269 0.15 0.5] Getting the Air Crystal
  (`|ExecutionSequence`
    (:`then_0`
      (`/Engine/EditorBlueprintResources/StandardMacros.DoOnce` false
        (:`Completed`
          (`GameplayStatics.PlaySound2D` (`self.Get_AirCrystal_SFX`) 1.0 1.0 0.0 null null))))
    (:`then_1`
      (bind _asbp_third_person_character (cast `/Game/Blueprints/BP_ThirdPersonCharacter` OtherActor))
      (`self.DisableInput` _asbp_third_person_character (`GameplayStatics.GetPlayerController` 0))
      (`/Game/Blueprints/BPI_Crystals.WindCrystalGet` _asbp_third_person_character)
      (`KismetSystemLibrary.Delay` 0.4)
      (message `/Game/Blueprints/BPI_Cloudbreak.BreakCloud` (`self.WhichCloud?`))
      (message `/Game/Blueprints/BPI_Cloudbreak.BreakCloud` (`self.WhichCloud?_2`))
      (`self.K2_DestroyActor`))))

(fn `UserConstructionScript`)