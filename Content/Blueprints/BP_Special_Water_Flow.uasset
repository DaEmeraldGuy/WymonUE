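; BP_Special_Water_Flow is a switchable water current that pushes the third-person character along its Arrow component's direction.
; Entering PushBox while the flow is enabled launches the character, and Tick offsets overlapping characters by Speed without sweeping.
; EnableFlow and DisableFlow triggers toggle pushing on any overlap, but switch the Floor's Pawn collision between Block and Ignore only for the character.
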(event `self.Disable Flow.OnComponentBeginOverlap`
  (params (OverlappedComponent :type "PrimitiveComponent Object Reference") (OtherActor :type "Actor Object Reference") (OtherComp :type "PrimitiveComponent Object Reference") (OtherBodyIndex :type Integer) (bFromSweep :type Boolean) (SweepResult :type "HitResult Structure (by ref)"))
  (set `self.Push Enable?` false)
  (cast `/Game/Blueprints/BP_ThirdPersonCharacter` OtherActor)
  (`PrimitiveComponent.SetCollisionResponseToChannel` (`self.Floor`) "ECC_Pawn" "ECR_Ignore"))

(event `self.Enable Flow.OnComponentBeginOverlap`
  (params (OverlappedComponent :type "PrimitiveComponent Object Reference") (OtherActor :type "Actor Object Reference") (OtherComp :type "PrimitiveComponent Object Reference") (OtherBodyIndex :type Integer) (bFromSweep :type Boolean) (SweepResult :type "HitResult Structure (by ref)"))
  (set `self.Push Enable?` true)
  (cast `/Game/Blueprints/BP_ThirdPersonCharacter` OtherActor)
  (`PrimitiveComponent.SetCollisionResponseToChannel` (`self.Floor`) "ECC_Pawn" "ECR_Block"))

(event `self.ReceiveTick`
  (params (DeltaSeconds :type "Float (single-precision)"))
  (if (`self.Push Enable?`)
    (for _array_element (`PrimitiveComponent.GetOverlappingActors` (`self.PushBox`) "/Game/Blueprints/BP_ThirdPersonCharacter.BP_ThirdPersonCharacter_C")
      (`self.K2_AddActorWorldOffset` _array_element (* (`KismetMathLibrary.GetForwardVector` (`SceneComponent.K2_GetComponentRotation` (`self.Arrow`))) (* DeltaSeconds (`self.Speed`))) false false))))

(event `self.PushBox.OnComponentBeginOverlap`
  (params (OverlappedComponent :type "PrimitiveComponent Object Reference") (OtherActor :type "Actor Object Reference") (OtherComp :type "PrimitiveComponent Object Reference") (OtherBodyIndex :type Integer) (bFromSweep :type Boolean) (SweepResult :type "HitResult Structure (by ref)"))
  (if (`self.Push Enable?`)
    (bind _asbp_third_person_character (cast `/Game/Blueprints/BP_ThirdPersonCharacter` OtherActor))
    (`Character.LaunchCharacter` _asbp_third_person_character (* (`KismetMathLibrary.Conv_RotatorToVector` (`SceneComponent.K2_GetComponentRotation` (`self.Arrow`))) 1000.0) false false)))

(fn `UserConstructionScript`)