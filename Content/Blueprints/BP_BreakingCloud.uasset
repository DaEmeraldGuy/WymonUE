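; BP_BreakingCloud is a cloud floor actor that breaks away once enough enemies are defeated.
; EventEnemiesDefeated increments a kill counter and, after a short delay, jumps into the BreakCloud sequence when it reaches four, with debug prints on each check.
; BreakCloud, also callable directly, waits briefly, plays a breaking sound and destroys the actor.
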(event `/Game/Blueprints/BPI_Cloudbreak.BreakCloud`
  (`KismetSystemLibrary.Delay` 0.8 :!label _label)
  (`GameplayStatics.PlaySound2D` (`self.Breaking_CloudFloor_SFX`) 1.0 1.0 0.0 null null)
  (`self.K2_DestroyActor`))

(event `EventEnemiesDefeated`
  (set `self.Enemies Killed` (+ (`self.Enemies Killed`) 1))
  (`KismetSystemLibrary.Delay` 0.2)
  (if (== (`self.Enemies Killed`) 4)
    (`KismetSystemLibrary.PrintString` "Is at 4")
    (goto _label)
    (else
      (`KismetSystemLibrary.PrintString` "Not at 4"))))

(fn `UserConstructionScript`)