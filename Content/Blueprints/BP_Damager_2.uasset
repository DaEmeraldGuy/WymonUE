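; BP_Damager_2 is a damage volume that hurts the third-person player character when it enters the box.
; On Box overlap it casts to BP_ThirdPersonCharacter and calls DecreasePlayerHealth with its DamgerDMG value.
; It then prints the damage and the character's current and max health as debug output.
; An ApplyDamage path is present but never wired to run.
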(event `self.Box.OnComponentBeginOverlap`
  (params (OverlappedComponent :type "PrimitiveComponent Object Reference") (OtherActor :type "Actor Object Reference") (OtherComp :type "PrimitiveComponent Object Reference") (OtherBodyIndex :type Integer) (bFromSweep :type Boolean) (SweepResult :type "HitResult Structure (by ref)"))
  (bind _damger_dmg (`self.Damger DMG`))
  ;[0.15 0 0 0.502] Damager (with "Decrease Player Health")
  (bind _asbp_third_person_character (cast `/Game/Blueprints/BP_ThirdPersonCharacter` OtherActor))
  (`/Game/Blueprints/BP_ThirdPersonCharacter.Decrease Player Health` _asbp_third_person_character _damger_dmg)
  (`KismetSystemLibrary.PrintString` (`KismetStringLibrary.Conv_IntToString` _damger_dmg))
  (`KismetSystemLibrary.PrintString` (`KismetTextLibrary.Conv_TextToString` (`|FormatText` "Player HP: {Current HP} / {Max HP}" (`/Game/Blueprints/BP_ThirdPersonCharacter.Player CurrentHealth` _asbp_third_person_character) (`/Game/Blueprints/BP_ThirdPersonCharacter.Player MaxHealth` _asbp_third_person_character))) true true (struct :`R` 0.000848 :`G` 0.270833 :`B` 0.035321 :`A` 1.0)))

(fn `UserConstructionScript`)