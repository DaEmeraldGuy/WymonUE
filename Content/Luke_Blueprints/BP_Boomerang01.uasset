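; Boomerang projectile that flies out, damages enemies and returns to the player character.
; A non-player overlap on its box, or a two-second timeout if not already returning, triggers BoomReturn; hits also spawn an effect and deal damage to BP_EnemyAI.
; BoomReturn zeroes gravity, then a timeline lerps it to the character's live Boomerang component position.
; When the timeline finishes, it destroys itself and calls ResetBoom on the character.
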(event `BoomReturn`
  (bind _asbp_third_person_character (cast `/Game/ThirdPerson/Blueprints/BP_ThirdPersonCharacter` (`GameplayStatics.GetPlayerCharacter` 0) :!pure true))
  (set `self.IsReturning` true)
  (set `ProjectileMovementComponent.ProjectileGravityScale` 0.0 (`self.ProjectileMovement`))
  (`KismetSystemLibrary.Delay` 0.1)
  (set `self.BoomLocBegin` (`self.K2_GetActorLocation` self))
  (bind (_direction _boomreturn) (`Timeline|BoomerangReturn`)
    (:`Update`
      (`self.K2_SetActorLocation` (`KismetMathLibrary.VLerp` (`self.BoomLocBegin`) (`SceneComponent.K2_GetComponentLocation` (`/Game/ThirdPerson/Blueprints/BP_ThirdPersonCharacter.Boomerang` _asbp_third_person_character)) _boomreturn)))
    (:`Finished`
      (`self.K2_DestroyActor`)
      (`/Game/ThirdPerson/Blueprints/BP_ThirdPersonCharacter.ResetBoom` _asbp_third_person_character))))

(event `self.ReceiveBeginPlay`
  (set `self.PlayerCharacter` (`GameplayStatics.GetPlayerPawn` (`self.Player Index`)))
  (`KismetSystemLibrary.Delay` 2.0)
  (if (not (`self.IsReturning`))
    (`self.BoomReturn`)))

(event `self.Box.OnComponentBeginOverlap`
  (params (OverlappedComponent :type "PrimitiveComponent Object Reference") (OtherActor :type "Actor Object Reference") (OtherComp :type "PrimitiveComponent Object Reference") (OtherBodyIndex :type Integer) (bFromSweep :type Boolean) (SweepResult :type "HitResult Structure (by ref)"))
  (bind (_asbp_enemy_ai _bsuccess) (cast `/Game/Luke_Blueprints/BP_EnemyAI` OtherActor :!pure true))
  (if (== OtherActor self)
    _
    (elif (not (== OtherActor (`GameplayStatics.GetPlayerCharacter` 0)))
      (`KismetSystemLibrary.PrintString` (`KismetSystemLibrary.GetDisplayName` OtherActor))
      (`|ExecutionSequence`
        (:`then_0`
          (`self.BoomReturn`))
        (:`then_1`
          (`NiagaraFunctionLibrary.SpawnSystemAtLocation` "/Game/Effects/BoomSystem.BoomSystem" (`self.K2_GetActorLocation`)))
        (:`then_2`
          (if _bsuccess
            (`KismetSystemLibrary.PrintString` "True")
            (`/Engine/EditorBlueprintResources/StandardMacros.IsValid` _asbp_enemy_ai
              (:`Is Valid`
                (`/Game/Luke_Blueprints/BP_EnemyAI.DecreaseHealth` _asbp_enemy_ai 100)))
            (else
              (`KismetSystemLibrary.PrintString` "False"))))))))

(fn `ReturnToPlayer`)

(fn `UserConstructionScript`)