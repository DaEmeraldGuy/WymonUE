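; Enemy AI Blueprint that chases the player once spotted and can be killed by damage.
; A PawnSensing component's sighting event sets a seen flag and triggers an AI MoveTo toward player character 0, regardless of which pawn was seen.
; The flag is never cleared in this Blueprint.
; A DecreaseHealth event subtracts damage and destroys the actor once health drops below zero.
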(event `self.PawnSensing.OnSeePawn`
  (params (Pawn :type "Pawn Object Reference"))
  (set `self.isSeeingPlayer` true)
  (`self.FollowPlayer`))

(event `FollowPlayer`
  (if (`self.isSeeingPlayer`)
    (`|AIMoveTo` self (0.0 0.0 0.0) (`GameplayStatics.GetPlayerCharacter` 0))))

(event `DecreaseHealth`
  (params (Damage :type Integer))
  (bind _output_get (set `self.Health` (- (`self.Health`) Damage)))
  (if (< _output_get 0)
    (`self.K2_DestroyActor`)))

(fn `UserConstructionScript`)