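; BP_CreamController is a controller that drives a 2D PaperZD player character with Enhanced Input.
; It adds the character input mapping context on BeginPlay, then routes left/right input to X-axis movement and jump input to Jump and StopJumping.
; On possession it binds to movement mode changes, jumping the animation state machine to the Airborne node when the character starts falling.
; The basic attack input is an empty stub.
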(event `self.ReceiveBeginPlay`
  (bind _returnvalue (subsystem `EnhancedInputLocalPlayerSubsystem`))
  (`/Engine/EditorBlueprintResources/StandardMacros.IsValid` _returnvalue
    (:`Is Valid`
      (`EnhancedInputSubsystemInterface.AddMappingContext` _returnvalue "/Game/Spritesheets/KeyMapping/IMC_CharacterInput.IMC_CharacterInput" 0 (struct)))))

(event `EnhancedInput|/Game/Spritesheets/KeyMapping/LeftRight`
  (params (ActionValue :type "Float (double-precision)") (ElapsedSeconds :type "Float (double-precision)") (TriggeredSeconds :type "Float (double-precision)") (InputAction :type "InputAction Object Reference" :default "/Game/Spritesheets/KeyMapping/LeftRight.LeftRight"))
  (:`Triggered`
    (`Pawn.AddMovementInput` (`GameplayStatics.GetPlayerCharacter` 0) (1.0 0.0 0.0) ActionValue false)))

(event `EnhancedInput|/Game/Spritesheets/KeyMapping/Jumping`
  (params (ActionValue :type "Float (double-precision)") (ElapsedSeconds :type "Float (double-precision)") (TriggeredSeconds :type "Float (double-precision)") (InputAction :type "InputAction Object Reference" :default "/Game/Spritesheets/KeyMapping/Jumping.Jumping"))
  (bind _returnvalue (`GameplayStatics.GetPlayerCharacter` 0))
  (:`Started`
    (`Character.Jump` _returnvalue))
  (:`Completed`
    (`Character.StopJumping` _returnvalue)))

(event `EnhancedInput|/Game/Spritesheets/KeyMapping/AttackBasic`
  (params (ActionValue :type Boolean) (ElapsedSeconds :type "Float (double-precision)") (TriggeredSeconds :type "Float (double-precision)") (InputAction :type "InputAction Object Reference" :default "/Game/Spritesheets/KeyMapping/AttackBasic.AttackBasic"))
  (:`Started`
    (if true
      _)))

(event `self.ReceivePossess`
  (params (PossessedPawn :type "Pawn Object Reference"))
  (add `Character.MovementModeChangedDelegate` (`GameplayStatics.GetPlayerCharacter` 0) (delegate `MovementModeChangedDelegate_Event`)))

(event `MovementModeChangedDelegate_Event`
  (params (Character :type "Character Object Reference") (PrevMovementMode :type "EMovementMode Enum" :default "MOVE_None") (PreviousCustomMode :type Byte))
  (bind _aspaper_zdcharacter (cast `PaperZDCharacter` Character))
  (switch `EMovementMode` (`CharacterMovementComponent.MovementMode` (`Character.CharacterMovement` Character))
    (:`MOVE_Falling`
      (`PaperZDAnimInstance.JumpToNode` (`PaperZDAnimationComponent.AnimInstance` (`PaperZDCharacter.AnimationComponent` _aspaper_zdcharacter)) "Airborne" "None"))))

(fn `UserConstructionScript`)