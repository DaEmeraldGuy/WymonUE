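; BP_Cream is a player-controlled character that can throw and spawn fireballs.
; On BeginPlay it adds the IMC_CharacterInput Enhanced Input mapping context to its player controller.
; The Throwing input action briefly raises the IsThrowing flag, then clears it after a delay.
; Separately, a hard-bound right mouse press spawns BP_Fireball at the actor's location and rotation, independent of that flag.
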(event `self.ReceiveBeginPlay`
  (bind _asplayer_controller (cast `PlayerController` (`self.GetController`)))
  (message `EnhancedInputSubsystemInterface.AddMappingContext` (pcsubsystem `EnhancedInputLocalPlayerSubsystem` _asplayer_controller) "/Game/Spritesheets/KeyMapping/IMC_CharacterInput.IMC_CharacterInput" 0 (struct)))

(event `EnhancedInput|/Game/Spritesheets/KeyMapping/Throwing`
  (params (ActionValue :type Boolean) (ElapsedSeconds :type "Float (double-precision)") (TriggeredSeconds :type "Float (double-precision)") (InputAction :type "InputAction Object Reference" :default "/Game/Spritesheets/KeyMapping/Throwing.Throwing"))
  (:`Triggered`
    (set `self.IsThrowing` true)
    (`KismetSystemLibrary.Delay` 0.5)
    (set `self.IsThrowing` false)))

(event `Key|RightMouseButton`
  (params (Key :type "Key Structure"))
  (:`Pressed`
    (`|SpawnActorFromClass` "/Game/Spritesheets/Blueprints/BP_Fireball.BP_Fireball_C" (`KismetMathLibrary.MakeTransform` (`self.K2_GetActorLocation`) (`self.K2_GetActorRotation`)) "Undefined" "MultiplyWithRoot" null null)))

(fn `UserConstructionScript`)