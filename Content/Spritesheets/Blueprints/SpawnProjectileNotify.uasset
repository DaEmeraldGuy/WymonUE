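; Animation notify that spawns an actor of a configurable class, by its name a projectile, when a sprite sequence fires it.
; The spawn transform derives from the render component's world transform, combined with the notify's Rotation and Scale, and ignores collisions.
; Both validity branches spawn identically, but only the invalid-owner branch, likely editor preview, can draw a debug bounds box when Debug is set.
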(fn `OnReceiveNotify`
  (params (OwningInstance :type "PaperZDAnimInstance Object Reference"))
  (bind (_origin _boxextent) (`KismetSystemLibrary.GetComponentBounds` null))
  (bind _class (`self.Class`))
  (bind (_returnvalue_location _returnvalue_rotation _returnvalue_scale) (`KismetMathLibrary.BreakTransform` (`SceneComponent.K2_GetComponentToWorld` (`self.SequenceRenderComponent`))))
  (bind _returnvalue (`KismetMathLibrary.MakeTransform` (+ _returnvalue_location (* (`KismetMathLibrary.GreaterGreater_VectorRotator` _returnvalue_location _returnvalue_rotation) _returnvalue_scale)) (`KismetMathLibrary.ComposeRotators` _returnvalue_rotation (`self.Rotation`)) (* (`self.Scale`) _returnvalue_scale)))
  (`/Engine/EditorBlueprintResources/StandardMacros.IsValid` OwningInstance
    (:`Is Valid`
      (`|SpawnActorFromClass` _class _returnvalue "AlwaysSpawn" "MultiplyWithRoot" null null))
    (:`Is Not Valid`
      (bind _returnvalue_2 (`|SpawnActorFromClass` _class _returnvalue "AlwaysSpawn" "MultiplyWithRoot" null null))
      (if (`self.Debug`)
        (`KismetSystemLibrary.DrawDebugBox` _origin _boxextent (struct) (`self.Rotation`))))))